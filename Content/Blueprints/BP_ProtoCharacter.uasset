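; BP_ProtoCharacter is a prototype character that performs 1-metre mantle up and mantle down moves.
; It binds to MantleComp's mantle-start event, prints the type and forwards it to the AnimInstance.
; During each move it blocks input and jumping, switches to Flying, disables capsule collision and ticks MantleComp.
; A hardcoded delay per mantle type then restores walking, input, collision and jumping, and stops the tick.
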(event Custom|Mantle
  (params (Type :type EMantleType%20Enum :default "Mantle2M"))
  (bind _returnvalue (Pawn|GetController))
  (bind _returnvalue_2 (Pawn|GetController))
  (Development|PrintString (Utilities|String|EnumtoString Type))
  (Class|Mantle|MantleSystem(Message) (Components|SkeletalMesh|GetAnimInstance (Variables|Character|GetMesh)) Type)
  (switch Utilities|FlowControl|Switch|SwitchonEMantleType Type
    (:Mantle1M
      (Utilities|FlowControl|Sequence
        (:then_0
          (Input|SetIgnoreLookInput _returnvalue true :!label _label)
          (Input|SetIgnoreMoveInput _returnvalue true)
          (Pawn|Components|CharacterMovement|SetMovementMode (Variables|Character|GetCharacterMovement) "MOVE_Flying" 0)
          (Collision|SetCollisionEnabled (Variables|Default|GetCapsuleComponent) "NoCollision")
          (bind _output_get (Variables|Default|SetbCanJump false))
          (Class|MantleComponent|SetTickEnabled (Variables|Default|GetMantleComp) (not _output_get)))
        (:then_1
          (Utilities|FlowControl|Delay (Math|Float|MakeLiteralFloat 1.67))
          (Input|SetIgnoreLookInput _returnvalue_2 false :!label _label_2)
          (Input|SetIgnoreMoveInput _returnvalue_2 false)
          (Pawn|Components|CharacterMovement|SetMovementMode (Variables|Character|GetCharacterMovement) "MOVE_Walking" 0)
          (Collision|SetCollisionEnabled (Variables|Default|GetCapsuleComponent) "QueryAndPhysics")
          (bind _output_get_2 (Variables|Default|SetbCanJump true))
          (Class|MantleComponent|SetTickEnabled (Variables|Default|GetMantleComp) (not _output_get_2)))))
    (:MantleDown1M
      (Utilities|FlowControl|Sequence
        (:then_0
          (goto _label))
        (:then_1
          (Utilities|FlowControl|Delay (Math|Float|MakeLiteralFloat 1.33))
          (goto _label_2))))))

(event EventBeginPlay
  (EventDispatchers|BindEventtoOnMantleStart (Variables|Default|GetMantleComp) (delegate Custom|Mantle)))

(fn ConstructionScript)